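; GameController Blueprint that links the main menu UI to the tile puzzle board.
; Once the UI is ready, it binds to the menu's restart button and the board's win delegate.
; Restart spawns tiles at the requested board size and randomizes them.
; A win only prints a message suggesting a larger tile count.
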(event Custom|RestartBtnClicked_Event_0
  (params (desiredBoardSize :type Integer))
  (Class|GameboardActor|SpawnTiles (Variables|Default|GetgameBoard) desiredBoardSize)
  (Class|GameboardActor|Randomize (Variables|Default|GetgameBoard)))

(event Custom|UIReady
  (EventDispatchers|AssignRestartBtnClicked (Variables|/Game/BluePrints/GameUIController.GameUIController_C|GetmainMenuUI (Variables|Default|GetgameUIController)) (delegate Custom|RestartBtnClicked_Event_0))
  (EventDispatchers|AssignOnWinDelegate (Variables|Default|GetgameBoard) (delegate Custom|OnWinDelegate_Event_1)))

(event Custom|OnWinDelegate_Event_1
  (Development|PrintString "You won! Try more tiles."))

(fn ConstructionScript)