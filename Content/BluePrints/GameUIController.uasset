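; GameUIController is a Blueprint that owns the game's main menu UI and toggles it on screen.
; On BeginPlay it enables input from player controller 0, creates a MainMenu widget, stores it, adds it to the viewport and calls UIInitialized.
; Pressing Q switches the stored widget between visible and hidden.
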(event EventBeginPlay
  (Input|EnableInput (Game|GetPlayerController 0))
  (bind _returnvalue (UserInterface|CreateWidget "/Game/BluePrints/MainMenu.MainMenu_C"))
  (bind _output_get (Variables|Default|SetmainMenuUI _returnvalue))
  (UserInterface|Viewport|AddtoViewport _output_get 0)
  (Default|CallUIInitialized))

(event Input|KeyboardEvents|Q
  (params (Key :type Key%20Structure :default "None"))
  (bind _mainmenuui (Variables|Default|GetmainMenuUI))
  (:Pressed
    (if (Widget|IsVisible (Variables|Default|GetmainMenuUI))
      (Widget|SetVisibility _mainmenuui "Hidden")
      (else
        (Widget|SetVisibility _mainmenuui "Visible")))))

(fn ConstructionScript)